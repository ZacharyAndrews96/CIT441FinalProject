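; First-person player character that damages targets with a flashlight in a timed, kill-goal stage, earning funds and supporting damage and speed upgrades.
; While lit, a per-tick camera trace sends damage messages; holding Attack focuses the beam for full damage but slows movement.
; Interact sends activation messages by trace.
; Tick also updates the countdown and checks kills, saving progress between stages or deleting the save upon final victory.
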(event EventBeginPlay
  (bind _returnvalue (UserInterface|CreateWidget "/Game/Widget/Counters.Counters_C"))
  (UserInterface|Viewport|AddtoViewport _returnvalue 0)
  (Variables|Default|SetCount _returnvalue)
  (bind _returnvalue_2 (SaveGame|DoesSaveGameExist "Data1"))
  (if _returnvalue_2
    (bind _returnvalue_3 (SaveGame|LoadGamefromSlot "Data1"))
    (bind _asdata (Utilities|Casting|CastToData _returnvalue_3))
    (Variables|Default|SetDamage (Variables|/Game/Blueprints/Data.Data_C|GetDamage _asdata))
    (Variables|Default|SetFunds (Variables|/Game/Blueprints/Data.Data_C|GetFunds _asdata))
    (Variables|Default|SetLevel (Variables|/Game/Blueprints/Data.Data_C|GetLevel _asdata))
    (bind _output_get (Variables|Default|SetSpeed (Variables|/Game/Blueprints/Data.Data_C|GetSpeed _asdata)))
    (Variables|/Script/Engine.CharacterMovementComponent|SetMaxWalkSpeed (Variables|Character|GetCharacterMovement) (Math|Conversions|ToFloat(Integer) _output_get))
    (else
      (bind _output_get_2 (Variables|/Script/Engine.CharacterMovementComponent|SetMaxWalkSpeed (Variables|Character|GetCharacterMovement) (Math|Conversions|ToFloat(Integer) (Variables|Default|GetSpeed))))))
  (Default|UpdateFunds (Variables|Default|GetCount) (Variables|Default|GetFunds))
  (Default|UpdateKills (Variables|Default|GetCount) (Variables|Default|GetKills))
  (Variables|Default|SetTimeLeft (Variables|Default|GetTimeLimit)))

(event Collision|EventActorBeginOverlap
  (params (OtherActor :type Actor%20Object%20Reference)))

(event EventTick
  (params (DeltaSeconds :type Float%20%28single-precision%29))
  (bind _camera (Variables|Default|GetCamera))
  (bind _returnvalue (Transformation|GetWorldLocation _camera))
  (Utilities|FlowControl|Sequence
    (:then_0
      (bind _output_get (Variables|Default|SetTimeLeft (- (Variables|Default|GetTimeLeft) DeltaSeconds)))
      (Default|UpdateTime (Variables|Default|GetCount) (Math|Float|Truncate _output_get))
      (if (>= (Variables|Default|GetTimeLeft) 0.0)
        (bind _returnvalue_2 (UserInterface|CreateWidget "/Game/Widget/Loss.Loss_C"))
        (UserInterface|Viewport|AddtoViewport _returnvalue_2 0)))
    (:then_1
      (bind _outhit (Collision|LineTraceByChannel _returnvalue (+ _returnvalue (* (Math|Vector|GetForwardVector _camera) (Variables|Default|GetAttackLimit))) "TraceTypeQuery1" false 0 "None"))
      (if (Variables|Default|GetLightOn)
        (if (Variables|Default|GetFullAttack)
          (Class|Damage|Damage(Message) (.hitactor _outhit) (Variables|Default|GetDamage))
          (else
            (Class|Damage|Damage(Message) (.hitactor _outhit) (/ (Variables|Default|GetDamage) 2))))))
    (:then_2
      (if (>= (Variables|Default|GetKills) (Variables|Default|GetGoals))
        (if (>= (Variables|Default|GetLevel) 2)
          (bind _returnvalue_3 (UserInterface|CreateWidget "/Game/Widget/Victory.Victory_C"))
          (UserInterface|Viewport|AddtoViewport _returnvalue_3 0)
          (SaveGame|DeleteGameinSlot "Data1")
          (Utilities|FlowControl|Delay 2.0)
          (Game|OpenLevel(byName) "MainMenu")
          (else
            (bind _returnvalue_4 (SaveGame|CreateSaveGameObject "/Game/Blueprints/Data.Data_C"))
            (Variables|/Game/Blueprints/Data.Data_C|SetDamage _returnvalue_4 (Variables|Default|GetDamage))
            (Variables|/Game/Blueprints/Data.Data_C|SetFunds _returnvalue_4 (Variables|Default|GetFunds))
            (Variables|/Game/Blueprints/Data.Data_C|SetLevel _returnvalue_4 (+ (Variables|Default|GetLevel) 1))
            (Variables|/Game/Blueprints/Data.Data_C|SetSpeed _returnvalue_4 (Variables|Default|GetSpeed))
            (SaveGame|SaveGametoSlot _returnvalue_4 "Data1")
            (bind _returnvalue_5 (UserInterface|CreateWidget "/Game/Widget/NextLevel.NextLevel_C"))
            (UserInterface|Viewport|AddtoViewport _returnvalue_5 0)
            (Utilities|FlowControl|Delay 2.0)
            (Game|OpenLevel(byName) "Stage")))))))

(event Input|ActionEvents|InputActionAttack
  (params (Key :type Key%20Structure :default "None"))
  (bind _charactermovement (Variables|Character|GetCharacterMovement))
  (bind _speed (Variables|Default|GetSpeed))
  (bind _spotlight (Variables|Default|GetSpotLight))
  (:Pressed
    (Rendering|Components|Light|SetIntensity _spotlight 5e+04)
    (Rendering|Lighting|SetOuterConeAngle _spotlight 15.0)
    (Variables|Default|SetFullAttack true)
    (Variables|/Script/Engine.CharacterMovementComponent|SetMaxWalkSpeed _charactermovement (Math|Conversions|ToFloat(Integer) (/ _speed 2)))
    (Audio|PlaySound2D "/Game/Audio/Click.Click" 1.0 1.0 0.0 0 0 :!label _label))
  (:Released
    (Rendering|Components|Light|SetIntensity _spotlight 5e+03)
    (Rendering|Lighting|SetOuterConeAngle _spotlight 3e+01)
    (Variables|Default|SetFullAttack false)
    (Variables|/Script/Engine.CharacterMovementComponent|SetMaxWalkSpeed _charactermovement (Math|Conversions|ToFloat(Integer) _speed))
    (goto _label)))

(event Input|ActionEvents|InputActionToggleLight
  (params (Key :type Key%20Structure :default "None")))

(event Input|ActionEvents|InputActionInteract
  (params (Key :type Key%20Structure :default "None"))
  (bind _camera (Variables|Default|GetCamera))
  (bind _returnvalue (Transformation|GetWorldLocation _camera))
  (:Pressed
    (bind _outhit (Collision|LineTraceByChannel _returnvalue (+ _returnvalue (* (Math|Vector|GetForwardVector _camera) (Variables|Default|GetInteractLimit))) "TraceTypeQuery1" false 0 "None"))
    (Class|Interact|Activate(Message) (.hitactor _outhit))))

(event Input|AxisEvents|InputAxisForward
  (params (AxisValue :type Float%20%28single-precision%29))
  (Class|PawnMovementComponent|AddInputVector (Variables|Character|GetCharacterMovement) (* (Transformation|GetActorForwardVector) AxisValue) true))

(event Input|AxisEvents|InputAxisStrafe
  (params (AxisValue :type Float%20%28single-precision%29))
  (Class|PawnMovementComponent|AddInputVector (Variables|Character|GetCharacterMovement) (* (Transformation|GetActorRightVector) AxisValue) true))

(event Input|AxisEvents|InputAxisViewSide
  (params (AxisValue :type Float%20%28single-precision%29))
  (Pawn|Input|AddControllerYawInput AxisValue))

(event Input|AxisEvents|InputAxisViewUp
  (params (AxisValue :type Float%20%28single-precision%29))
  (bind _camera (Variables|Default|GetCamera))
  (bind _returnvalue (Transformation|GetWorldRotation _camera))
  (bind _returnvalue_2 (+ AxisValue (.pitch _returnvalue)))
  (if (not (>= (Math|Float|Absolute(Float) _returnvalue_2) 3e+01))
    (Transformation|SetWorldRotation _camera (Math|Rotator|MakeRotator 0.0 _returnvalue_2 (.yaw _returnvalue)) false false)))

(fn ConstructionScript)

(fn AddKill
  (bind _output_get (Variables|Default|SetKills (+ (Variables|Default|GetKills) 1)))
  (Default|UpdateKills (Variables|Default|GetCount) _output_get)
  (CallFunction|ChangeFunds 5))

(fn UpgradeDamage
  (Variables|Default|SetDamage (+ (Variables|Default|GetDamage) 2)))

(fn UpgradeSpeed
  (bind _output_get (Variables|Default|SetSpeed (+ (Variables|Default|GetSpeed) 100)))
  (Variables|/Script/Engine.CharacterMovementComponent|SetMaxWalkSpeed (Variables|Character|GetCharacterMovement) (Math|Conversions|ToFloat(Integer) _output_get)))

(fn ChangeFunds
  (params (Amount :type Integer))
  (bind _output_get (Variables|Default|SetFunds (+ (Variables|Default|GetFunds) Amount)))
  (Default|UpdateFunds (Variables|Default|GetCount) _output_get))