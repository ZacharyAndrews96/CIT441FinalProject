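; GhostLove is an AI ghost pawn that wanders randomly and can have a lover that mourns its death.
; Damage starts an invulnerability cooldown, plays a burn sound and temporarily shifts the material by health lost.
; Tick handles cooldown, faces movement direction and, at zero health, credits the player's kill, notifies Love and destroys the ghost.
; A notified lover changes color, moves near the death spot and repeatedly plays a crying sound.
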(event Custom|wander
  (AI|AIMoveTo self (.RandomLocation (AI|Navigation|GetRandomReachablePointinRadius (Transformation|GetActorLocation) 1e+03 0 0)) 0 5.0 false
    (:OnSuccess
      _)
    (:OnFail
      _))
  (CallFunction|Wander))

(event Custom|movetoLover
  (AI|AIMoveTo self (.RandomLocation (AI|Navigation|GetRandomReachablePointinRadius (Variables|Default|GetGoal) 1e+03 0 0)) 0 5.0 false
    (:OnSuccess
      _)
    (:OnFail
      _))
  (CallFunction|Cry))

(event Custom|Cry
  (Audio|PlaySoundatLocation "/Game/Audio/Why.Why" (Transformation|GetActorLocation) "0, 0, 0" 1.0 1.0 0.0 "/Game/Audio/WhyAttention.WhyAttention" 0 0)
  (Utilities|FlowControl|Delay 3.0)
  (CallFunction|Cry))

(event EventBeginPlay
  (CallFunction|Wander)
  (Development|PrintString "Hello i'm spawned in"))

(event Collision|EventActorBeginOverlap
  (params (OtherActor :type Actor%20Object%20Reference)))

(event EventTick
  (params (DeltaSeconds :type Float%20%28single-precision%29))
  (bind _love (Variables|Default|GetLove))
  (Utilities|FlowControl|Sequence
    (:then_0
      (if (>= (Variables|Default|GetCoolDown) 0.0)
        (Variables|Default|SetCoolDown (- (Variables|Default|GetCoolDown) DeltaSeconds))
        (else
          (Rendering|Material|SetScalarParameterValueonMaterials (Variables|Default|GetStaticMesh) "Lerp" 0.0))))
    (:then_1
      (if (> (Math|Vector|VectorLength (Transformation|GetVelocity)) 0.5)
        (Transformation|SetActorRotation (Math|Rotator|MakeRotfromX (Variables|/Script/Engine.MovementComponent|GetVelocity (Variables|Default|GetFloatingPawnMovement))) true)))
    (:then_2
      (if (<= (Variables|Default|GetHealth) 0)
        (Audio|SpawnSoundatLocation "/Game/Audio/NO.NO" (Transformation|GetActorLocation) "0, 0, 0" 1.0 1.0 0.0 0 0)
        (bind _asadventure_character (Utilities|Casting|CastToAdventureCharacter (Game|Player|GetPlayerPawn 0)))
        (Default|AddKill _asadventure_character)
        (Utilities|IsValid _love
          (:Is%20Valid
            (CallFunction|LookforLover _love (Transformation|GetActorLocation)))
          (:Is%20Not%20Valid
            _))
        (Actor|DestroyActor)))))

(event EventDamage
  (params (Dam :type Integer))
  (if (not (>= (Variables|Default|GetCoolDown) 0.0))
    (Variables|Default|SetCoolDown 2.5)
    (bind _output_get (Variables|Default|SetHealth (- (Variables|Default|GetHealth) Dam)))
    (if (> _output_get 0)
      (Audio|SpawnSoundatLocation "/Game/Audio/LightBurns.LightBurns" (Transformation|GetActorLocation) "0, 0, 0" 1.0 1.0 0.0 0 0)
      (bind _output_get_2 (Variables|Default|SetScalarValue (- 1.0 (/ (Math|Conversions|ToFloat(Integer) (Variables|Default|GetHealth)) (Math|Conversions|ToFloat(Integer) (Variables|Default|GetStartingHealth))))))
      (Rendering|Material|SetScalarParameterValueonMaterials (Variables|Default|GetStaticMesh) "Lerp" _output_get_2))))

(fn ConstructionScript
  (bind _output_get (Variables|Default|SetHealth (Variables|Default|GetMaxHealth)))
  (Variables|Default|SetStartingHealth _output_get)
  (Variables|/Script/Engine.FloatingPawnMovement|SetMaxSpeed (Variables|Default|GetFloatingPawnMovement) (Variables|Default|GetSpeed)))

(fn SetupPostSpawn
  (params (Health :type Integer) (Speed :type Float%20%28single-precision%29))
  (bind _output_get (Variables|Default|SetHealth Health))
  (Variables|Default|SetStartingHealth _output_get)
  (Variables|Default|SetSpeed Speed))

(fn LookforLover
  (params (Death%20Spot :type Vector))
  (Variables|Default|SetGoal Death%20Spot)
  (CallFunction|MovetoLover)
  (Rendering|Material|SetVectorParameterValueonMaterials (Variables|Default|GetStaticMesh) "Color" "0.344000,0.322000,0.755000")
  (Development|PrintString "Death of lover"))