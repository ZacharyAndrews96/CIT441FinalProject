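; TrapSound is an actor that plays a sound once when the player comes within range.
; Each Tick it compares the distance between the first player's pawn and itself against Range.
; The first time that check passes, it sets an Activated flag, plays the Sound at its location and deactivates its particle system.
; The flag is never reset here, so the trigger does not repeat.
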(event EventBeginPlay)

(event Collision|EventActorBeginOverlap
  (params (OtherActor :type Actor%20Object%20Reference)))

(event EventTick
  (params (DeltaSeconds :type Float%20%28single-precision%29))
  (if (< (Math|Vector|Distance(Vector) (Transformation|GetActorLocation (Game|Player|GetPlayerPawn 0)) (Transformation|GetActorLocation)) (Variables|Default|GetRange))
    (if (not (Variables|Default|GetActivated))
      (Variables|Default|SetActivated true)
      (Audio|PlaySoundatLocation (Variables|Default|GetSound) (Transformation|GetActorLocation) "0, 0, 0" 1.0 1.0 0.0 0 0 0)
      (Components|Activation|Deactivate (Variables|Default|GetParticleSystem)))))

(fn ConstructionScript)