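; TrapSpawn is a one-shot proximity trap that spawns a basic ghost when the player comes near.
; Each tick it compares the player pawn's distance to Range and, the first time inside, sets Activated and plays a sound at its location.
; It then spawns a GhostBasic at a random reachable nav point nearby, initializes its health and speed, and deactivates its particle system.
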(event EventBeginPlay)

(event Collision|EventActorBeginOverlap
  (params (OtherActor :type Actor%20Object%20Reference)))

(event EventTick
  (params (DeltaSeconds :type Float%20%28single-precision%29))
  (bind _returnvalue (Transformation|GetActorLocation))
  (if (< (Math|Vector|Distance(Vector) (Transformation|GetActorLocation (Game|Player|GetPlayerPawn 0)) (Transformation|GetActorLocation)) (Variables|Default|GetRange))
    (if (not (Variables|Default|GetActivated))
      (Variables|Default|SetActivated true)
      (Audio|PlaySoundatLocation (Variables|Default|GetSound) _returnvalue "0, 0, 0" 1.0 1.0 0.0 0 0 0)
      (bind _returnvalue_2 (Game|SpawnActorfromClass "/Game/Blueprints/GhostBasic.GhostBasic_C" (Math|Transform|MakeTransform (.RandomLocation (AI|Navigation|GetRandomReachablePointinRadius _returnvalue 5e+02 0 0)) "0, 0, 0" "1,1,1") "Undefined" 0 0))
      (Default|SetupPostSpawn _returnvalue_2 1 2e+02)
      (Components|Activation|Deactivate (Variables|Default|GetParticleSystem)))))

(fn ConstructionScript)